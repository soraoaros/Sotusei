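; Short-lived chemical effect actor that toggles a Niagara component's "SpawnStop" flag on timed delays.
; BeginPlay waits briefly, sets the flag true, then gives the actor a limited life span so it destroys itself.
; Tick runs through a longer delay that sets the flag false, repeating for as long as the actor lives.
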(event `self.ReceiveBeginPlay`
  (`KismetSystemLibrary.Delay` 1.1)
  (set `self.NewVar_0` true)
  (`NiagaraComponent.SetVariableBool` (`self.Niagara`) "SpawnStop" (`self.NewVar_0`))
  (`self.SetLifeSpan` 11.0))

(event `self.ReceiveTick`
  (params (DeltaSeconds :type "Float (single-precision)"))
  (`KismetSystemLibrary.Delay` 2.7)
  (set `self.NewVar_0` false)
  (`NiagaraComponent.SetVariableBool` (`self.Niagara`) "SpawnStop" (`self.NewVar_0`)))

(fn `UserConstructionScript`)