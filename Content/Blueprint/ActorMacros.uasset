(fn `UserConstructionScript`
  (`parent.UserConstructionScript`))