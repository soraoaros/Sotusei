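; AI controller for an enemy that detects the player and escalates through idle, warning, threat, pursuit, fast approach and battle states.
; Tick raises or decays an alert value from perception sight and alert-area checks; crossing the maximum triggers pursuit or a one-shot threat.
; Attack range switches between battle and a randomly chosen pursuit style, with State written to the Blackboard driving BT_Enemy.
; It sends chase flags to the player and stops the tree on death.
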(event `self.ReceivePossess`
  (params (PossessedPawn :type "Pawn Object Reference"))
  (bind _blackboard (`self.Blackboard`))
  (`self.RunBehaviorTree` "/Game/Enemy/AI/BT_Enemy.BT_Enemy") ; ビヘイビアツリー呼び出し
  (`BlackboardComponent.SetValueAsObject` _blackboard "selfActor" (`self.K2_GetPawn`)) ; BB値セット
  (`BlackboardComponent.SetValueAsObject` _blackboard "isHit" (`self.K2_GetPawn`)))

(event `self.AIPerception.OnPerceptionUpdated`
  (params (UpdatedActors :type "Array of Actor Object Reference (by ref)"))
  (bind _isalive (`self.HealthCheck`)) ; 生きているかの確認
  (if _isalive
    ;[1 1 1] Playerに対する視界情報のアップデートかを判定
    (for _array_element UpdatedActors
      (if (== _array_element (`GameplayStatics.GetPlayerCharacter` 0))
        ;[1 1 1] 視界に入った・出たの判定
        (bind _info (`AIPerceptionComponent.GetActorsPerception` (`self.AIPerception`) _array_element))
        (if (`.bSuccessfullySensed` (break `AIStimulus` (`|GetArrayItem` (`.LastSensedStimuli` (break `ActorPerceptionBlueprintInfo` _info)))))
          (set `self.isInSight` true) ; 視界に入ったかのフラグ
          (`KismetSystemLibrary.PrintString` "InSight")
          (else
            (set `self.isInSight` false) ; 視界から出た
            (`KismetSystemLibrary.PrintString` "OutSight")))))))

(event `/Game/Enemy/Interfaces/BPI_EnemyController.SetAlertValue`
  (params (alertvalue :type "Float (single-precision)"))
  ;[1 1 1] AlertValueセット
  (set `self.alertValue` alertvalue))

(event `/Game/Enemy/Interfaces/BPI_EnemyController.SetAlertMagnification`
  (params (magnification :type "Float (single-precision)"))
  ;[1 1 1] AlertValueセット
  (set `self.Magnification` magnification))

(event `self.ReceiveTick`
  (params (DeltaSeconds :type "Float (single-precision)"))
  ;[1 1 1] 生存確認
  (bind _isalive (`self.HealthCheck`))
  (if _isalive
    (`self.SetBattleORPursuit`) ; 戦闘できそうならセット
    ;[1 1 1] Stateの振り分け
    (bind _result (`self.UpdateAlertValue` (* (`self.Magnification`) DeltaSeconds))) ; 発見していればTrueが返ってくる
    (if _result
      (if (`|EnumEquality` (`self.State`) "NewEnumerator1")
        (message `/Game/Enemy/Interfaces/BPI_Enemy.StateChangeWarning` (`self.K2_GetPawn`) false) ; 警戒中でない
        (`self.Pursuit Start`) ; 追跡開始
        (else
          (`/Engine/EditorBlueprintResources/StandardMacros.DoOnce` false :!label _label
            (:`Completed`
              (`self.SetThreat`) ; 威嚇
              (`BlackboardComponent.SetValueAsEnum` (`self.Blackboard`) "State" (`self.State`) :!label _label_2) ; Stateをセット
            ))))
      (elif (> (`self.alertValue`) 0.0)
        (`self.SetWarning`) ; 警戒
        (`self.SetBBLengthWithTarget`)
        (goto _label_2)
        (else
          (`self.SetIdle`) ; 待機
          (`self.ThreatReset`) ; 威嚇リセット
          (goto _label_2))))
    (else
      (`/Engine/EditorBlueprintResources/StandardMacros.DoOnce` false
        (:`Completed`
          ;[1 1 1] HPが0以下の場合、ビヘイビアツリーを停止する
          (set `self.State` "NewEnumerator6")
          (message `/Game/Player/BPI_Player.SetIsChase` (`GameplayStatics.GetPlayerCharacter` 0) false) ; プレイヤーにchaseフラグ送信
          (`BrainComponent.StopLogic` (`self.BrainComponent`) "dead"))))))

(event `/Game/Enemy/Interfaces/BPI_EnemyController.SetBattle`
  ;[1 1 1] Stateの振り分け
  (set `self.State` "NewEnumerator4")
  (`KismetSystemLibrary.PrintString` "戦闘中" true false (struct :`R` 1.0 :`G` 0.135651 :`A` 1.0))
  (goto _label_2))

(event `/Game/Enemy/Interfaces/BPI_EnemyController.SetFastApproach`
  ;[1 1 1] Stateの振り分け
  (`self.SetPursuitFast`)
  (goto _label_2))

(event `ThreatReset`
  ;[1 1 1] Stateの振り分け
  (goto _label :!via `Reset`))

(event `/Game/Enemy/Interfaces/BPI_EnemyController.FastApproachEnd`
  ;[1 1 1] Stateの振り分け
  (`self.SetPursuit` :!label _label_3) ; 追跡
  (goto _label_2))

(event `/Game/Enemy/Interfaces/BPI_EnemyController.ThreatEnd`
  ;[1 1 1] Stateの振り分け
  (message `/Game/Player/BPI_Player.SetIsChase` (`GameplayStatics.GetPlayerCharacter` 0) true :!label _label_4) ; プレイヤーにchaseフラグ送信
  (switch `int` (`KismetMathLibrary.RandomIntegerInRange` 0 1)
    (:`0`
      (goto _label_3))
    (:`1`
      (`self.SetPursuitFast` :!label _label_5) ; 急接近
      (goto _label_2))))

(event `Pursuit Start`
  ;[1 1 1] Stateの振り分け
  (goto _label_4))

(event `/Game/Enemy/Interfaces/BPI_EnemyController.HitHeadShot`
  ;[1 1 1] Stateの振り分け
  ;;[1 1 1] HS時に歩き状態なら
  (if (`|EnumEquality` (`self.State`) "NewEnumerator2")
    (goto _label_5)))

(fn `GetLengthWithTarget`
  (returns (Length :type "Float (double-precision)"))
  (bind _returnvalue (`KismetMathLibrary.VSize` (- (`self.K2_GetActorLocation` (`GameplayStatics.GetPlayerCharacter` 0)) (`self.K2_GetActorLocation` (`self.K2_GetPawn`)))))
  (`KismetSystemLibrary.PrintString` (`KismetStringLibrary.Concat_StrStr` "TargetDistance:" (`KismetStringLibrary.Conv_DoubleToString` _returnvalue)) true true (struct :`R` 0.135557 :`G` 1.0 :`B` 0.920299 :`A` 1.0) 0.01)
  (return _returnvalue))

(fn `HealthCheck`
  (returns (isAlive :type Boolean))
  ;[1 1 1] HPチェック
  (bind _health (message `/Game/Enemy/Interfaces/BPI_Enemy.GetHealth` (`self.K2_GetPawn`)))
  (return (> _health 0.0)))

(fn `SetBattleORPursuit`
  (bind _state (`self.State`))
  (if (`|EnumInequality` (`self.State`) "NewEnumerator6")
    ;[1 1 1] 攻撃範囲チェック
    (bind _length (`self.GetLengthWithTarget`))
    (bind (_attackrange _isattack _isgrab) (message `/Game/Enemy/Interfaces/BPI_Enemy.GetBattleParam` (`self.K2_GetPawn`)))
    (if (> _attackrange _length)
      (if (and (`|EnumInequality` _state "NewEnumerator4") (or (`|EnumEquality` _state "NewEnumerator2") (`|EnumEquality` _state "NewEnumerator7")))
        ;[1 1 1] State変更
        (`KismetSystemLibrary.PrintString` "戦闘中" true false (struct :`R` 1.0 :`G` 0.135651 :`A` 1.0))
        (set `self.State` "NewEnumerator4")
        (`BlackboardComponent.SetValueAsEnum` (`self.Blackboard`) "State" (`self.State`) :!label _label) ; Stateをセット
      )
      (elif (or _isattack _isgrab)
        _
        (elif (`|EnumEquality` (`self.State`) "NewEnumerator4")
          (switch `int` (`KismetMathLibrary.RandomIntegerInRange` 0 1)
            (:`0`
              (`self.SetPursuit`) ; 追跡
              (goto _label))
            (:`1`
              (`self.SetPursuitFast`) ; 急接近
              (goto _label))))))))

(fn `SetBBLengthWithTarget`
  (bind _length (`self.GetLengthWithTarget`))
  (`BlackboardComponent.SetValueAsFloat` (`self.Blackboard`) "lengthWithTarget" _length)
  (return))

(fn `SetIdle`
  (if (`|EnumInequality` (`self.State`) "NewEnumerator0")
    (`KismetSystemLibrary.PrintString` "待機中" true false (struct :`G` 1.0 :`A` 1.0))
    (set `self.State` "NewEnumerator0")
    (message `/Game/Enemy/Interfaces/BPI_Enemy.StateChangeWarning` (`self.K2_GetPawn`) false) ; 警戒中
    (message `/Game/Player/BPI_Player.SetIsChase` (`GameplayStatics.GetPlayerCharacter` 0) false) ; プレイヤーにchaseフラグ送信
  ))

(fn `SetPursuit`
  (`KismetSystemLibrary.PrintString` "追跡" (`|EnumInequality` (`self.State`) "NewEnumerator2") false (struct :`R` 1.0 :`A` 1.0))
  (set `self.State` "NewEnumerator2")
  (`BlackboardComponent.SetValueAsObject` (`self.Blackboard`) "targetActor" (`GameplayStatics.GetPlayerCharacter` 0)) ; BBにTargetActorをセット
)

(fn `SetPursuitFast`
  (`KismetSystemLibrary.PrintString` "追跡：急接近" (`|EnumInequality` (`self.State`) "NewEnumerator7") false (struct :`R` 1.0 :`A` 1.0))
  (set `self.State` "NewEnumerator7")
  (`BlackboardComponent.SetValueAsObject` (`self.Blackboard`) "targetActor" (`GameplayStatics.GetPlayerCharacter` 0)) ; BBにTargetActorをセット
)

(fn `SetThreat`
  (`KismetSystemLibrary.PrintString` "威嚇" (`|EnumInequality` (`self.State`) "NewEnumerator3") false (struct :`R` 1.0 :`G` 0.529659 :`B` 0.47384 :`A` 1.0))
  (set `self.State` "NewEnumerator3")
  (message `/Game/Enemy/Interfaces/BPI_Enemy.ThreatStart` (`self.K2_GetPawn`))
  (return))

(fn `SetWarning`
  (if (`|EnumInequality` (`self.State`) "NewEnumerator1")
    (`KismetSystemLibrary.PrintString` "警戒中" true false (struct :`R` 1.0 :`G` 1.0 :`A` 1.0))
    (set `self.State` "NewEnumerator1")
    (message `/Game/Enemy/Interfaces/BPI_Enemy.StateChangeWarning` (`self.K2_GetPawn`) true) ; 警戒中
    (message `/Game/Player/BPI_Player.SetIsChase` (`GameplayStatics.GetPlayerCharacter` 0) false) ; プレイヤーにchaseフラグ送信
  ))

(fn `UpdateAlertValue`
  (params (delta :type "Float (double-precision)"))
  (returns (result :type Boolean))
  (bind _alertvalue (`self.alertValue`))
  (bind _is_in_alert_area (message `/Game/Enemy/Interfaces/BPI_Enemy.GetIsInAlertArea` (`self.K2_GetPawn`)))
  (if (or (or (`self.isInSight`) _is_in_alert_area) (`self.isLost`))
    (set `self.alertValue` (+ delta (`self.alertValue`))) ; 警戒中は増やす
    (return (> (`self.alertValue`) (`self.MaxAlertValue`)))
    (elif (and (> _alertvalue 0.0) (`|EnumInequality` (`self.State`) "NewEnumerator3"))
      (set `self.alertValue` (- _alertvalue delta)) ; 警戒していなければ減らす
      (return (> (`self.alertValue`) (`self.MaxAlertValue`))))))

(fn `UserConstructionScript`)