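; Parent zombie enemy character that handles damage, death, loot and persistence, exposing combat state and notifying its AI controller.
; Point damage triggers per-bone physical-animation flinches, traced blood decals and headshot alerts, with brief invincibility limiting health loss.
; Death plays a directional montage, rolls weighted drops that favor whichever healing item the player lacks, and optionally queues a respawn.
; Alive/dead state saves by object name in GameInstance, removing dead enemies on continue.
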(event `self.ReceiveBeginPlay`
  (set `self.InitTransform` (`self.GetTransform`)) ; 初期Transform保持
  (bind _returnvalue (`GameplayStatics.GetActorOfClass` "/Game/FirstPersonBP/Blueprints/Object/PC/BP_SavePC.BP_SavePC_C"))
  (`/Engine/EditorBlueprintResources/StandardMacros.IsValid` _returnvalue
    (:`Is Valid`
      (add `/Game/FirstPersonBP/Blueprints/Object/PC/BP_SavePC.Save` _returnvalue (delegate `save`)))
    (:`Is Not Valid`
      _))
  (`self.LoadData`))

(event `save`
  (`self.SaveData`))

(event `self.ReceiveTick`
  (params (DeltaSeconds :type "Float (single-precision)"))
  (`self.UpdateInvincibleTime` DeltaSeconds) ; 無敵時間更新
  (`self.UpdateAttackCD` DeltaSeconds) ; 攻撃CD更新
  (`self.UpdateThreatTime` DeltaSeconds) ; 威嚇タイマー
)

(event `self.ReceivePointDamage`
  (params (Damage :type "Float (single-precision)") (DamageType :type "DamageType Object Reference") (HitLocation :type "Vector Structure") (HitNormal :type "Vector Structure") (HitComponent :type "PrimitiveComponent Object Reference") (BoneName :type Name) (ShotFromDirection :type "Vector Structure") (InstigatedBy :type "Controller Object Reference") (DamageCauser :type "Actor Object Reference") (HitInfo :type "HitResult Structure (by ref)"))
  ;[1 1 1] ダメージを受けたとき
  ;;[1 1 1] 変数保持
  (set `self.hitLocation` HitLocation)
  (bind _output_get (set `self.Bone Name` BoneName))
  (`self.HSCheck` _output_get)
  (set `self.shotDirection` (- (`self.K2_GetActorLocation` (`GameplayStatics.GetPlayerCharacter` 0)) (`self.hitLocation`)))
  (`self.SpawnDamageEffects`) ; Effect生成
  (`self.SetDamagePhysicalAnimation`) ; PhysicsAnimatoin呼び出し
  (if (> (`self.health`) 0.0)
    (if (not (> (`self.invincibleTime`) 0.0))
      (`self.TakeDamageProcess` Damage) ; ダメージ処理
      ;;[1 1 1] 死亡時の処理
      (if (<= (`self.health`) 0.0)
        (bind _returnvalue (`GameplayStatics.GetActorOfClass` "/Game/FirstPersonBP/Blueprints/FirstPersonCharacter.FirstPersonCharacter_C"))
        (`/Engine/EditorBlueprintResources/StandardMacros.IsValid` _returnvalue ; Actorが使える状態かどうか判断\nこれやらないと、FPCTutorial入れてない時に\nエラー吐く\nIsNotValidを先につなげる
          (:`Is Valid`
            (set `/Game/FirstPersonBP/Blueprints/FirstPersonCharacter.EnemyDeathTutorialFlag` true _returnvalue))
          (:`Is Not Valid`
            _))
        (`self.SaveDestroy`)
        (bind _deathmotionlength (`self.DeathProcess`))
        (`KismetSystemLibrary.Delay` (`KismetMathLibrary.RandomFloatInRange` (+ _deathmotionlength 1.8) (+ _deathmotionlength 2.4)))
        (`self.K2_DestroyActor`) ; 削除
      ))))

(event `SetDamagePhysicalAnimation`
  ;[1 1 1] PhysicalAnimation(部位がぶるぶる揺れるやつ)
  (if (!= (`self.Bone Name`) "Hip_J")
    (`PhysicalAnimationComponent.SetSkeletalMeshComponent` (`self.PhysicalAnimation`) (`self.Mesh`))
    (`PhysicalAnimationComponent.ApplyPhysicalAnimationSettingsBelow` (`self.PhysicalAnimation`) (`self.Bone Name`) (make `PhysicalAnimationData` true 1000.0 100.0 1000.0 100.0) true)
    (`SkeletalMeshComponent.SetAllBodiesBelowSimulatePhysics` (`self.Mesh`) (`self.Bone Name`) true true)
    (`|ExecutionSequence`
      (:`then_0`
        (bind (_direction _blendweight) (`Timeline|タイムライン_0` :!via `PlayFromStart`)
          (:`Update`
            (`SkeletalMeshComponent.SetAllBodiesBelowPhysicsBlendWeight` (`self.Mesh`) (`self.Bone Name`) _blendweight false true))
          (:`Finished`
            (`SkeletalMeshComponent.SetAllBodiesSimulatePhysics` (`self.Mesh`) false))))
      (:`then_1`
        (`PrimitiveComponent.AddImpulse` (`self.Mesh`) (* (`self.shotDirection`) (`KismetMathLibrary.RandomFloatInRange` -15.0 -5.0)) (`self.Bone Name`) false)))))

(event `SpawnFloorBlood`
  (bind _hitlocation (`self.hitLocation`))
  ;[1 0 0.06745] 出血デカール：StaticMeshのみ
  ;;[1 1 1] 地面に血を付ける処理
  (bind (_returnvalue _location _normal _rotation) (`self.Find Spawn Decal Point` _hitlocation (- _hitlocation (`KismetMathLibrary.MakeVector` 0.0 0.0 (`self.ZTraceLength`))) (`self.Object Types`)))
  (if _returnvalue
    (`|SpawnActorFromClass` "/Game/Effects/BP/BP_FloorBlood.BP_FloorBlood_C" (`KismetMathLibrary.MakeTransform` _location _rotation) "Undefined" "OverrideRootScale" null null)))

(event `SpawnWallBlood`
  (bind _hitlocation (`self.hitLocation`))
  (bind (_x _y _z) (`self.SetVectorVariation` (`self.Min`) (`self.Max`)))
  ;[1 0 0.06745] 出血デカール：StaticMeshのみ
  ;;[1 1 1] 壁に血を出す
  (bind (_returnvalue _location _normal _rotation) (`self.Find Spawn Decal Point` _hitlocation (+ _hitlocation (+ (* (`self.GetActorForwardVector` (`GameplayStatics.GetPlayerController` 0)) (`self.TraceLength`)) (`KismetMathLibrary.MakeVector` _x _y _z))) (`self.Object Types`)))
  (if _returnvalue
    (if (> (`KismetMathLibrary.DegAcos` (`KismetMathLibrary.Dot_VectorVector` _normal (0.0 0.0 1.0))) 40.0)
      (`|SpawnActorFromClass` "/Game/Effects/BP/BP_WallBlood.BP_WallBlood_C" (`KismetMathLibrary.MakeTransform` _location _rotation) "Undefined" "OverrideRootScale" null null))))

(event `self.Box(AlertAreaCollision).OnComponentBeginOverlap`
  (params (OverlappedComponent :type "PrimitiveComponent Object Reference") (OtherActor :type "Actor Object Reference") (OtherComp :type "PrimitiveComponent Object Reference") (OtherBodyIndex :type Integer) (bFromSweep :type Boolean) (SweepResult :type "HitResult Structure (by ref)"))
  ;[1 1 1] 警戒エリア用の判定
  (if (`/Game/Macro/Macro_CheckTags.CheckTags` OtherComp "Player")
    (bind (_outhit _returnvalue) (`KismetSystemLibrary.LineTraceSingle` :`Start` (`self.K2_GetActorLocation`) :`End` (`SceneComponent.K2_GetComponentLocation` OtherComp) :`TraceChannel` "TraceTypeQuery2" :`DrawDebugType` "ForDuration")) ; プレイヤーに向けてレイを飛ばす
    (if _returnvalue
      (if (== (`.HitComponent` (`GameplayStatics.BreakHitResult` _outhit)) OtherComp)
        (set `self.isInAlertArea` true)))))

(event `/Game/Enemy/Interfaces/BPI_Enemy.SetAttackMotionFlag`
  (params (flag :type Boolean))
  ;[0 1 0.4198] BPI関連
  ;;[1 1 1] 攻撃モーションフラグセット
  (set `self.inAttackMotion` flag))

(event `/Game/Enemy/Interfaces/BPI_Enemy.SetAttackCollisionFlag`
  (params (flag :type Boolean))
  ;[0 1 0.4198] BPI関連
  ;;[1 1 1] 攻撃判定セット
  (set `self.isAttackCollision` flag))

(event `self.Box(AlertAreaCollision).OnComponentEndOverlap`
  (params (OverlappedComponent :type "PrimitiveComponent Object Reference") (OtherActor :type "Actor Object Reference") (OtherComp :type "PrimitiveComponent Object Reference") (OtherBodyIndex :type Integer))
  ;[1 1 1] 警戒エリア用の判定
  (if (`/Game/Macro/Macro_CheckTags.CheckTags` OtherComp "Player")
    (set `self.isInAlertArea` false)))

(event `/Game/Enemy/Interfaces/BPI_Enemy.DeadNotify`
  ;[0 1 0.4198] BPI関連
  ;;[1 1 1] 死亡通知
  (`self.Spawn Item`) ; アイテム生成
)

(fn `Approach`
  (params (Fast :type Boolean))
  (returns (AcceptanceRadius :type "Float (double-precision)"))
  (set `self.isFastApproach` Fast)
  (set `CharacterMovementComponent.MaxWalkSpeed` (`KismetMathLibrary.SelectFloat` 250.0 100.0 Fast) (`self.CharacterMovement`))
  (return (- (`KismetMathLibrary.SelectFloat` 250.0 100.0 Fast) 70.0)))

(fn `ApproachResult`
  (params (ApproachResult :type "EPathFollowingRequestResult Enum" :default "Failed"))
  (returns (Result :type Boolean))
  (if (and (`|EnumEquality` ApproachResult "AlreadyAtGoal") (`self.isFastApproach`))
    (message `/Game/Enemy/Interfaces/BPI_EnemyController.FastApproachEnd` (`AIBlueprintHelperLibrary.GetAIController` self))
    (return false)))

(fn `DeathProcess`
  (returns (DeathMotionLength :type "Float (double-precision)"))
  (locals (DeathAnimLength :type "Float (double-precision)"))
  (`self.SendSpawner`)
  (bind _animlength (`self.SwitchDeathAnimation`)) ; 死亡アニメーション遷移
  (set `local.DeathAnimLength` _animlength)
  (set `self.deathLocation` (`SceneComponent.K2_GetComponentLocation` (`self.Mesh`))) ; 死亡場所を保存
  (`PrimitiveComponent.SetCollisionEnabled` (`self.CapsuleComponent`) "NoCollision")
  (`PrimitiveComponent.SetCollisionEnabled` (`self.Sphere(AttackCollision)`) "NoCollision")
  (`PrimitiveComponent.SetCollisionEnabled` (`self.Box(AlertAreaCollision)`) "NoCollision") ; 判定消す
  ;[1 1 1] アイテム処理
  (bind _result (`self.SetRandomDropItem`)) ; DropItemセット
  (if _result
    (`self.DropItemSpawn`) ; Item生成
  )
  (if (`self.isRespawn`)
    ;[1 1 1] Managerに変数追加
    (`EnemyManagerHelperBase.AddSpawnParam` (`EnemyManager.SubsystemHelper` (subsystem `EnemyManager`)) (`self.InitTransform`) "None" (`self.ItemNum`)))
  (return (`local.DeathAnimLength`)))

(fn `DropItemSpawn`
  (`KismetSystemLibrary.PrintString` (`KismetStringLibrary.Concat_StrStr` "アイテム名：" (`KismetStringLibrary.Conv_NameToString` (`self.ItemName`)) "/ 個数：" (`KismetStringLibrary.Conv_DoubleToString` (`self.ItemNum`))) true true (struct :`G` 1.0 :`B` 0.061222 :`A` 1.0) 3.0)
  (`|SpawnActorFromClass` "/Game/FirstPersonBP/Blueprints/Item/BP_ItemBase.BP_ItemBase_C" (`self.GetTransform`) "Undefined" "OverrideRootScale" null (`self.ItemName`) (`self.ItemNum`) true 1.0 (0.0 0.0 100.0) true null))

(fn `Find Spawn Decal Point`
  (params (Start :type "Vector Structure") (End :type "Vector Structure") (ObjectTypes :type "Array of EObjectTypeQuery Enum"))
  (returns (ReturnValue :type Boolean) (Location :type "Vector Structure") (Normal :type "Vector Structure") (Rotation :type "Rotator Structure"))
  (bind (_outhit _returnvalue) (`KismetSystemLibrary.LineTraceSingleForObjects` :`Start` Start :`End` End :`ObjectTypes` ObjectTypes :`DrawDebugType` "ForDuration"))
  (bind (_bblockinghit _binitialoverlap _time _distance _location _impactpoint _normal) (`GameplayStatics.BreakHitResult` _outhit))
  (return _returnvalue _location _normal (`KismetMathLibrary.FindLookAtRotation` _impactpoint (+ _impactpoint (- _normal -90.0)))))

(fn `GetActorLocation`
  (returns (location :type "Vector Structure"))
  (return (`self.K2_GetActorLocation`)))

(fn `GetAnimStateParam`
  (returns (Health :type "Float (double-precision)") (isFastApproach :type Boolean) (isWarning :type Boolean) (deathDirection :type "Vector Structure"))
  (return (`self.health`) (`self.isFastApproach`) (`self.isWarning`) (`self.shotDirection`)))

(fn `GetBattleParam`
  (returns (AttackRange :type "Float (double-precision)") (isAttack :type Boolean) (isGrab :type Boolean))
  (return (`self.AttackRange`) (`self.isAttack`) (`self.isGrabAttackCollision`)))

(fn `GetHealth`
  (returns (health :type "Float (double-precision)"))
  (return (`self.health`)))

(fn `GetIsInAlertArea`
  (returns (`is in Alert Area` :type Boolean))
  (return (`self.isInAlertArea`)))

(fn `HSCheck`
  (params (boneName :type Name))
  (if (or (== boneName "Head_J") (== boneName "Neck_J"))
    (message `/Game/Enemy/Interfaces/BPI_EnemyController.HitHeadShot` (`AIBlueprintHelperLibrary.GetAIController` self))))

(fn `LoadData`
  (bind _asbp_game_instance (cast `/Game/SaveData/BP_GameInstance` (`GameplayStatics.GetGameInstance`) :!pure true))
  (bind (_value _returnvalue) (`BlueprintMapLibrary.Map_Find` (`/Game/SaveData/BP_GameInstance.EnemyData` _asbp_game_instance) (`KismetSystemLibrary.GetObjectName` self)))
  (if (not (`/Game/SaveData/BP_GameInstance.IsHajimekara` _asbp_game_instance))
    (if _returnvalue
      (if (not (`.IsSonzai_1_92D2290B4E2A7B7B0EDC7E9D8DBFFA34` (break `/Game/SaveData/Str_EnemyData` _value)))
        (if (`self.isRespawn`)
          (`EnemyManagerHelperBase.AddSpawnParam` (`EnemyManager.SubsystemHelper` (subsystem `EnemyManager`)) (`self.InitTransform`) "None" (`self.ItemNum`)))
        (`self.K2_DestroyActor`)))))

(fn `SaveData`
  (bind _returnvalue (`KismetSystemLibrary.GetObjectName` self))
  (bind _enemydata (`/Game/SaveData/BP_GameInstance.EnemyData` (cast `/Game/SaveData/BP_GameInstance` (`GameplayStatics.GetGameInstance`) :!pure true)))
  (if (`.ReturnValue` (`BlueprintMapLibrary.Map_Find` _enemydata _returnvalue))
    (`BlueprintMapLibrary.Map_Remove` _enemydata _returnvalue))
  (`BlueprintMapLibrary.Map_Add` _enemydata (`KismetSystemLibrary.GetObjectName` self) (make `/Game/SaveData/Str_EnemyData` true)))

(fn `SaveDestroy`
  (bind _returnvalue (`KismetSystemLibrary.GetObjectName` self))
  (bind _enemydata (`/Game/SaveData/BP_GameInstance.EnemyData` (cast `/Game/SaveData/BP_GameInstance` (`GameplayStatics.GetGameInstance`) :!pure true)))
  (if (`.ReturnValue` (`BlueprintMapLibrary.Map_Find` _enemydata _returnvalue))
    (`BlueprintMapLibrary.Map_Remove` _enemydata _returnvalue))
  (`BlueprintMapLibrary.Map_Add` _enemydata (`KismetSystemLibrary.GetObjectName` self) (make `/Game/SaveData/Str_EnemyData` false)))

(fn `SendSpawner`
  ;[1 1 1] 親は何もしない
)

(fn `SetDropRate`
  (params (dropRate :type "Array of /Game/Enemy/Str_ItemDropRate Structure (by ref)"))
  (returns (result :type "Array of /Game/Enemy/Str_ItemDropRate Structure"))
  (bind _returnvalue (`GameplayStatics.GetPlayerCharacter` 0))
  (bind _output (`|GetArrayItem` dropRate 2))
  (bind _output_2 (`|GetArrayItem` dropRate 1))
  ;[1 1 1] ハーブと薬液の所持数チェック
  (bind (_is _num) (message `/Game/Player/BPI_Player.BPI_SearchInventoryItem` _returnvalue "Yaku"))
  (bind (_is_2 _num_2) (message `/Game/Player/BPI_Player.BPI_SearchInventoryItem` _returnvalue "Potion"))
  (if (== _num _num_2)
    ;[1 1 1] 薬液、ハーブの確率セット
    (setmembers `/Game/Enemy/Str_ItemDropRate` :`StructRef` _output_2 :`dropRate` 0.1)
    (setmembers `/Game/Enemy/Str_ItemDropRate` :`StructRef` _output :`dropRate` 0.1)
    (else
      (bind _returnvalue_2 (> _num _num_2))
      (setmembers `/Game/Enemy/Str_ItemDropRate` :`StructRef` _output_2 :`dropRate` (`KismetMathLibrary.SelectFloat` 0.15 0.05 _returnvalue_2))
      (setmembers `/Game/Enemy/Str_ItemDropRate` :`StructRef` _output :`dropRate` (`KismetMathLibrary.SelectFloat` 0.05 0.15 _returnvalue_2))))
  (return dropRate))

(fn `SetRandomDropItem`
  (returns (result :type Boolean))
  (locals (TotalRate :type "Float (double-precision)") (RandomPoint :type "Float (double-precision)") (StrItemDropRate :type "Array of /Game/Enemy/Str_ItemDropRate Structure") (resultName :type Name))
  (if (!= (`self.ItemName`) "None")
    (bind _result (`self.SetDropRate` (`local.StrItemDropRate`))) ; 薬液とハーブの確率セット
    (bind _output_get (set `local.StrItemDropRate` _result))
    (for _array_element _output_get
      (set `local.TotalRate` (+ (`local.TotalRate`) (`.dropRate_4_DF4828D2446B6CF896550396CA23B902` (break `/Game/Enemy/Str_ItemDropRate` _array_element)))) ; ローカル変数\nアイテム毎の抽選率を合計
    )
    (set `local.RandomPoint` (* (`KismetMathLibrary.RandomFloat`) (`local.TotalRate`))) ; 各アイテムの総ドロップ率の範囲でランダム
    (for _array_element_2 (`local.StrItemDropRate`)
      (bind (_dropitemname _droprate) (break `/Game/Enemy/Str_ItemDropRate` _array_element_2))
      (if (< (`local.RandomPoint`) _droprate)
        (bind _output_get_2 (set `local.resultName` _dropitemname))
        (switch `name` _output_get_2
          (:`Default`
            (set `self.ItemName` (`local.resultName`))
            (set `self.ItemNum` 1.0)
            (return true))
          (:`Gunpowder`
            (set `self.ItemName` (`local.resultName`))
            (set `self.ItemNum` (`KismetMathLibrary.Conv_IntToDouble` (`KismetMathLibrary.RandomIntegerInRange` 1 4))))
          (:`Gunpowder7`
            (set `self.ItemName` "Gunpowder")
            (set `self.ItemNum` 7.0))
          (:`None`
            (return false)))
        (return true)
        (else
          (set `local.RandomPoint` (- (`local.RandomPoint`) _droprate)))))))

(fn `SetVectorVariation`
  (params (Min :type "Float (double-precision)") (Max :type "Float (double-precision)"))
  (returns (X :type "Float (double-precision)") (Y :type "Float (double-precision)") (Z :type "Float (double-precision)"))
  (return (`KismetMathLibrary.RandomFloatInRange` Min Max) (`KismetMathLibrary.RandomFloatInRange` Min Max) (`KismetMathLibrary.RandomFloatInRange` Min Max)))

(fn `Spawn Item`
  (if (> (`self.ItemNum`) 0.0)
    (`|SpawnActorFromClass` "/Game/FirstPersonBP/Blueprints/Item/BP_ItemBase.BP_ItemBase_C" (`KismetMathLibrary.MakeTransform` (`SceneComponent.GetSocketLocation` (`self.Mesh`) "ItemSpawnSocket")) "Undefined" "OverrideRootScale" null (`self.ItemName`) (`self.ItemNum`) true 1.0 (0.0 0.0 100.0) false null)
    (return)))

(fn `SpawnDamageEffects`
  (bind (_returnvalue_roll _returnvalue_pitch _returnvalue_yaw) (`KismetMathLibrary.BreakRotator` (`self.K2_GetActorRotation` (`GameplayStatics.GetPlayerController` 0))))
  ;[1 1 1] 出血エフェクト生成
  (`NiagaraFunctionLibrary.SpawnSystemAtLocation` "/Game/Niagara/NS_BodyBloodImpact.NS_BodyBloodImpact" (`self.hitLocation`) (`KismetMathLibrary.MakeRotator` (+ _returnvalue_roll 180.0) _returnvalue_pitch (+ _returnvalue_yaw 180.0)))
  ;[1 1 1] 地面と壁に血を付ける
  (`self.SpawnFloorBlood`)
  (`self.SpawnWallBlood`))

(fn `SwitchDeathAnimation`
  (returns (AnimLength :type "Float (double-precision)"))
  (locals (Length :type "Float (double-precision)"))
  (bind _degree (`self.CalcAngle` (`self.GetActorForwardVector`) (`self.shotDirection`)))
  (if (and (>= _degree 45.0) (<= _degree 135.0))
    (bind _returnvalue (`self.PlayAnimMontage` "/Game/Enemy/Character/Animations_Zombie/Zombie_Death_Left_Montage.Zombie_Death_Left_Montage")) ; 左
    (set `local.Length` _returnvalue)
    (elif (and (>= _degree -135.0) (<= _degree -45.0))
      (bind _returnvalue_2 (`self.PlayAnimMontage` "/Game/Enemy/Character/Animations_Zombie/Zombie_Death_Right_Montage.Zombie_Death_Right_Montage")) ; 右
      (set `local.Length` _returnvalue_2)
      (elif (and (<= _degree 90.0) (>= _degree -90.0))
        (bind _returnvalue_3 (`self.PlayAnimMontage` "/Game/Enemy/Character/Animations_Zombie/Zombie_Death_Back_Montage.Zombie_Death_Back_Montage")) ; 後ろ
        (set `local.Length` _returnvalue_3)
        (else
          (bind _returnvalue_4 (`self.PlayAnimMontage` "/Game/Enemy/Character/Animations_Zombie/Zombie_Death_Front_Montage.Zombie_Death_Front_Montage")) ; 前
          (set `local.Length` _returnvalue_4)))))
  (return (`local.Length`)))

(fn `TakeDamageProcess`
  (params (damage :type "Float (double-precision)"))
  (set `self.isHit` true)
  (set `self.invincibleTime` 0.1) ; 無敵時間セット
  (set `self.health` (- (`self.health`) damage))
  (message `/Game/Enemy/Interfaces/BPI_EnemyController.SetAlertValue` (`AIBlueprintHelperLibrary.GetAIController` self) 6.0)
  (`GameplayStatics.PlaySoundAtLocation` (select `bool` (> (`self.health`) 0.0) :`false` "/Game/Enemy/Sounds/Cue_ZombieDead.Cue_ZombieDead" :`true` "/Game/Enemy/Sounds/Cue_ZombieNoise.Cue_ZombieNoise" :!type "SoundBase Object Reference") (`SceneComponent.K2_GetComponentLocation` (`self.Sphere(AttackCollision)`)) (struct) 1.0 1.0 0.0 null null null) ; うめき声
  (return))

(fn `UpdateAttackCD`
  (params (delta :type "Float (double-precision)"))
  (bind _attackcd (`self.attackCD`))
  (if (`self.isAttack`)
    (if (> _attackcd 0.0)
      (set `self.attackCD` (- _attackcd delta))
      (else
        (set `self.isAttack` false)
        (set `self.attackCD` -1.0)))))

(fn `UpdateInvincibleTime`
  (params (delta :type "Float (double-precision)"))
  (bind _invincibletime (`self.invincibleTime`))
  (if (`self.isHit`)
    (if (> _invincibletime 0.0)
      (set `self.invincibleTime` (- _invincibletime delta))
      (else
        (set `self.isHit` false) ; 無敵終了でフラグ消す
      ))))

(fn `UpdateThreatTime`
  (params (Delta :type "Float (double-precision)"))
  (if (> (`self.ThreatTime`) 0.0)
    (bind _output_get (set `self.ThreatTime` (- (`self.ThreatTime`) Delta))) ; Delta減らす
    (if (> 0.0 _output_get)
      (set `self.isThreat` false)
      (message `/Game/Enemy/Interfaces/BPI_EnemyController.ThreatEnd` (`AIBlueprintHelperLibrary.GetAIController` self)) ; 終了
    )))

(fn `UserConstructionScript`)