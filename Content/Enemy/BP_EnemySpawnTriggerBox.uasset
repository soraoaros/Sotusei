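; Trigger box that respawns enemies when a component tagged Player overlaps it.
; It copies saved transforms, item names and item counts from the EnemyManager subsystem helper, then spawns a BP_Enemy per transform with its matching item data, flagged as a respawn.
; It then clears both its local arrays and the manager's saved params, so each saved set spawns only once.
; Tick draws the box bounds for debugging.
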(event `self.ReceiveTick`
  (params (DeltaSeconds :type "Float (single-precision)"))
  (bind _box (`self.Box`))
  ;[0.3524 1 0.4819] Debug
  (`KismetSystemLibrary.DrawDebugBox` (`SceneComponent.K2_GetComponentLocation` _box) (`BoxComponent.BoxExtent` _box) (struct :`R` 0.415625 :`G` 0.502261 :`B` 1.0 :`A` 1.0) (`SceneComponent.K2_GetComponentRotation` _box)))

(event `self.Box.OnComponentBeginOverlap`
  (params (OverlappedComponent :type "PrimitiveComponent Object Reference") (OtherActor :type "Actor Object Reference") (OtherComp :type "PrimitiveComponent Object Reference") (OtherBodyIndex :type Integer) (bFromSweep :type Boolean) (SweepResult :type "HitResult Structure (by ref)"))
  ;[1 1 1] Enemy生成処理
  (if (`/Game/Macro/Macro_CheckTags.CheckTags` OtherComp "Player")
    (`self.SaveSpawnParam`)
    (for (_array_element _array_index) (`self.SpawnTransform`)
      (`|SpawnActorFromClass` "/Game/Enemy/BP_Enemy.BP_Enemy_C" _array_element "AlwaysSpawn" "OverrideRootScale" null (`|GetArrayItem` (`self.SpawnItemName`) _array_index) (`|GetArrayItem` (`self.SpawnItemNum`) _array_index) true null))
    (`KismetArrayLibrary.Array_Clear` (`self.SpawnTransform`)) ; 保持していた配列のクリア
    (`KismetArrayLibrary.Array_Clear` (`self.SpawnItemName`))
    (`KismetArrayLibrary.Array_Clear` (`self.SpawnItemNum`))
    (`EnemyManagerHelperBase.ClearSpawnParams` (`EnemyManager.SubsystemHelper` (subsystem `EnemyManager`)))))

(fn `SaveSpawnParam`
  ;[1 1 1] EnemyManagerから値取得
  (bind (_transforms _names _nums) (`EnemyManagerHelperBase.GetSpawnParams` (`EnemyManager.SubsystemHelper` (subsystem `EnemyManager`))))
  (set `self.SpawnTransform` _transforms)
  (set `self.SpawnItemName` _names)
  (set `self.SpawnItemNum` _nums)
  (return))

(fn `UserConstructionScript`)