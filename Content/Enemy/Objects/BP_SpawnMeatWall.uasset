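; Meat wall spawner actor that spawns a BP_Enemy at its spawn point when a Player-tagged component enters its trigger box.
; Each spawn disarms it and starts a cooldown set in minutes, which Tick counts down.
; It re-arms only once the cooldown has elapsed and the previously spawned enemy is no longer valid.
; The construction script disables collision on the two meat wall mesh components.
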(event `self.ReceiveTick`
  (params (DeltaSeconds :type "Float (single-precision)"))
  (`parent.ReceiveTick` DeltaSeconds)
  (`self.UpdateCoolDown` DeltaSeconds) ; CD更新
)

(event `self.SpawnTriggerBox.OnComponentBeginOverlap`
  (params (OverlappedComponent :type "PrimitiveComponent Object Reference") (OtherActor :type "Actor Object Reference") (OtherComp :type "PrimitiveComponent Object Reference") (OtherBodyIndex :type Integer) (bFromSweep :type Boolean) (SweepResult :type "HitResult Structure (by ref)"))
  ;[1 1 1] 生成処理
  (if (and (`/Game/Macro/Macro_CheckTags.CheckTags` OtherComp "Player") (`self.waitingForSpawn`))
    (bind _returnvalue (`|SpawnActorFromClass` "/Game/Enemy/BP_Enemy.BP_Enemy_C" (`SceneComponent.K2_GetComponentToWorld` (`self.SpawnPoint`)) "AlwaysSpawn" "OverrideRootScale" null "None" 0.0 false null))
    (set `self.SpawnEnemy` _returnvalue)
    (set `self.waitingForSpawn` false)
    (set `self.spawnCoolDown` (* 60.0 (`self.SpawnCD`)))))

(fn `UpdateCoolDown`
  (params (delta :type "Float (double-precision)"))
  (if (> (`self.spawnCoolDown`) 0.0)
    (set `self.spawnCoolDown` (- (`self.spawnCoolDown`) delta)) ; 更新
    (else
      (`/Engine/EditorBlueprintResources/StandardMacros.IsValid` (`self.SpawnEnemy`) ; 存在するか
        (:`Is Not Valid`
          (if (not (`self.waitingForSpawn`))
            (set `self.waitingForSpawn` true)))))))

(fn `UserConstructionScript`
  (`parent.UserConstructionScript`)
  (`PrimitiveComponent.SetCollisionEnabled` (`self.meatwall_pPlane136`) "NoCollision")
  (`PrimitiveComponent.SetCollisionEnabled` (`self.meatwall_pCube1058`) "NoCollision"))