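; Enemy actor Blueprint that takes point damage and attacks the player when its Attack event is called, per comments by AI.
; Point damage outside a short invincibility window reduces Health, spawns a Niagara blood impact at the hit location, and destroys the actor at zero health.
; Attack applies damage directly to player character 0 without a hit check (marked provisional) and plays an animation.
; Tick counts down invincibility and attack cooldown, clearing IsHit and IsAttack afterward.
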(event `self.ReceiveTick`
  (params (DeltaSeconds :type "Float (single-precision)"))
  (`self.UpdateInvincibleTime` DeltaSeconds) ; 無敵時間更新
  (`self.UpdateAttackCD` DeltaSeconds) ; 攻撃のCD更新
)

(event `self.ReceivePointDamage`
  (params (Damage :type "Float (single-precision)") (DamageType :type "DamageType Object Reference") (HitLocation :type "Vector Structure") (HitNormal :type "Vector Structure") (HitComponent :type "PrimitiveComponent Object Reference") (BoneName :type Name) (ShotFromDirection :type "Vector Structure") (InstigatedBy :type "Controller Object Reference") (DamageCauser :type "Actor Object Reference") (HitInfo :type "HitResult Structure (by ref)"))
  ;[1 1 1] ダメージを受けたとき
  (set `self.Damage` Damage)
  (set `self.Hit Location` HitLocation)
  (if (not (> (`self.invincibleTime`) 0.0))
    (set `self.isHit` true)
    (set `self.invincibleTime` 0.1) ; 無敵時間セット
    (bind _output_get (set `self.health` (- (`self.health`) (`self.Damage`))))
    (`NiagaraFunctionLibrary.SpawnSystemAtLocation` "/Game/Niagara/NS_BodyBloodImpact.NS_BodyBloodImpact" (`self.Hit Location`))
    (if (<= _output_get 0.0)
      (`self.K2_DestroyActor`) ; 消去する
    )))

(event `/Game/Enemy/Interfaces/BP_EnemyAIInterface.Attack`
  ;[1 1 1] AIから攻撃の信号が送られてきたら動く攻撃処理
  (if (not (`self.isAttack`))
    (set `self.isAttack` true)
    (`GameplayStatics.ApplyDamage` (`GameplayStatics.GetPlayerCharacter` 0) 1.0) ; 仮：当たり判定とってやりたい
    (`SkeletalMeshComponent.PlayAnimation` (`self.Mesh`) "/Game/Enemy/Animations/Silly_Dancing_Anim_mixamo_com.Silly_Dancing_Anim_mixamo_com" false)
    (set `self.attackCD` 3.0) ; 攻撃可能まで3秒くらい
  ))

(fn `UpdateAttackCD`
  (params (deltaSeconds :type "Float (double-precision)"))
  (bind _attackcd (`self.attackCD`))
  (if (> _attackcd 0.0)
    (set `self.attackCD` (- _attackcd deltaSeconds))
    (else
      (set `self.isAttack` false) ; 攻撃可能にする
    )))

(fn `UpdateInvincibleTime`
  (params (deltaSeconds :type "Float (double-precision)"))
  (bind _invincibletime (`self.invincibleTime`))
  (if (> _invincibletime 0.0)
    (set `self.invincibleTime` (- _invincibletime deltaSeconds)) ; 無敵時間を更新する
    (else
      (set `self.isHit` false) ; 無敵終了でフラグ消す
    )))

(fn `UserConstructionScript`)