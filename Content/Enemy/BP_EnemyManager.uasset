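; BP_EnemyManager stores timed spawn entries, presumably for enemies, as parallel arrays of transform, item name, count, cooldown and readiness flag.
; AddSpawnParam appends an entry with a fixed starting cooldown, not yet spawnable, while Get, Set and Clear handle all arrays together.
; UpdateSpawnCoolDown subtracts the passed delta from positive cooldowns and flags expired entries as spawnable.
; The spawning itself is not performed here.
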(fn `AddSpawnParam`
  (params (transform :type "Transform Structure (by ref)") (name :type "Name (by ref)") (num :type "Float (double-precision) (by ref)"))
  (`KismetArrayLibrary.Array_Add` (`self.SpawnTransforms`) transform)
  (`KismetArrayLibrary.Array_Add` (`self.SpawnItemNames`) name)
  (`KismetArrayLibrary.Array_Add` (`self.SpawnItemNums`) num)
  (`KismetArrayLibrary.Array_Add` (`self.SpawnCoolDowns`) 180.0)
  (`KismetArrayLibrary.Array_Add` (`self.SpawnIsPossibles`))
  (return))

(fn `ClearSpawnParams`
  (`KismetArrayLibrary.Array_Clear` (`self.SpawnTransforms`))
  (`KismetArrayLibrary.Array_Clear` (`self.SpawnItemNames`))
  (`KismetArrayLibrary.Array_Clear` (`self.SpawnItemNums`))
  (`KismetArrayLibrary.Array_Clear` (`self.SpawnCoolDowns`))
  (`KismetArrayLibrary.Array_Clear` (`self.SpawnIsPossibles`)))

(fn `GetSpawnParams`
  (returns (transforms :type "Array of Transform Structure") (names :type "Array of Name") (nums :type "Array of Float (double-precision)") (spawnCD :type "Array of Float (double-precision)") (isPossible :type "Array of Boolean"))
  (return (`self.SpawnTransforms`) (`self.SpawnItemNames`) (`self.SpawnItemNums`) (`self.SpawnCoolDowns`) (`self.SpawnIsPossibles`)))

(fn `SetSpawnParams`
  (params (transforms :type "Array of Transform Structure (by ref)") (names :type "Array of Name (by ref)") (nums :type "Array of Float (double-precision) (by ref)") (spawnCD :type "Array of Float (double-precision) (by ref)") (isPossible :type "Array of Boolean (by ref)"))
  (set `self.SpawnTransforms` transforms)
  (set `self.SpawnItemNames` names)
  (set `self.SpawnItemNums` nums)
  (set `self.SpawnCoolDowns` spawnCD)
  (set `self.SpawnIsPossibles` isPossible))

(fn `UpdateSpawnCoolDown`
  (params (delta :type "Float (double-precision) (by ref)"))
  (for (_array_element _array_index) (`self.SpawnCoolDowns`)
    (if (> _array_element 0.0)
      (`KismetArrayLibrary.Array_Set` (`self.SpawnCoolDowns`) _array_index (- _array_element delta))
      (else
        (`KismetArrayLibrary.Array_Set` (`self.SpawnIsPossibles`) _array_index true)))))